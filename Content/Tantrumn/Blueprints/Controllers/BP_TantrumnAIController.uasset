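; AI controller for Tantrumn that runs the BT_TantrumnBattle behavior tree and feeds it level and match state.
; On BeginPlay it starts the tree and stores the location of the first TantrumnLevelEndTrigger found as the Destination blackboard vector.
; Each tick it writes the game state's IsPlaying result to a blackboard bool, though that key name is set to None.
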(event `self.ReceiveBeginPlay`
  (`self.RunBehaviorTree` "/Game/Tantrumn/Blueprints/AI/Behavior_Trees/BT_TantrumnBattle.BT_TantrumnBattle")
  (bind _outactors (`GameplayStatics.GetAllActorsOfClass` "/Script/Tantrumn.TantrumnLevelEndTrigger"))
  (if (> (`KismetArrayLibrary.Array_Length` _outactors) 0)
    (`BlackboardComponent.SetValueAsVector` (`self.Blackboard`) "Destination" (`self.K2_GetActorLocation` (`|GetArrayItem` _outactors)))))

(event `self.ReceiveTick`
  (params (DeltaSeconds :type "Float (single-precision)"))
  (bind _astantrumn_game_state_base (cast `TantrumnGameStateBase` (`GameplayStatics.GetGameState`)))
  (`BlackboardComponent.SetValueAsBool` (`self.Blackboard`) "None" (`TantrumnGameStateBase.IsPlaying` _astantrumn_game_state_base)))

(fn `UserConstructionScript`)